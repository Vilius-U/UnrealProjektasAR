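; Mocap mannequin actor that plays looping animations and makes short lane-style sidesteps and jumps.
; A touch press runs a MultiGate through walk, run and crouch-walk animations, while a separate function plays a one-shot cheerful walk.
; MoveLeft, MoveRight and Jump events lerp the actor's location along forward or up vectors via timelines.
; Left, right, middle and jumping flags track state, with middle detected at the world origin.
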(event `Key|Touch1`
  (params (Key :type "Key Structure"))
  (bind _sk_mannequin (`self.SK_Mannequin`))
  (:`Pressed`
    (`|MultiGate` false :!label _label
      (:`Out 0`
        (`SkeletalMeshComponent.PlayAnimation` _sk_mannequin "/Game/MCO_Mocap_Basics/Animation/Mobility_Pro/In_Place/MOB1_Walk_F_IPC.MOB1_Walk_F_IPC" true))
      (:`Out 1`
        (`SkeletalMeshComponent.PlayAnimation` _sk_mannequin "/Game/MCO_Mocap_Basics/Animation/Mobility_Pro/In_Place/MOB1_Run_F_IPC.MOB1_Run_F_IPC" true))
      (:`Out 2`
        (`SkeletalMeshComponent.PlayAnimation` _sk_mannequin "/Game/MCO_Mocap_Basics/Animation/Mobility_Pro/In_Place/MOB1_CrouchWalk_F_IPC.MOB1_CrouchWalk_F_IPC" true)
        (goto _label :!via `Reset`)))))

(event `MoveLeft`
  ;[1 1 1] Moving to left
  (bind _output_get (set `self.StartLocation` (`self.K2_GetActorLocation`)))
  (bind _output_get_2 (set `self.TargetLocation` (+ _output_get (* (`self.GetActorForwardVector`) (10.0 10.0 10.0)))))
  (bind (_direction _newtrack_0) (`Timeline|MoveLeftTimeline` :!via `PlayFromStart`)
    (:`Update`
      (`self.K2_SetActorLocation` (`KismetMathLibrary.VLerp` _output_get _output_get_2 _newtrack_0)))
    (:`Finished`
      (set `self.IsMovedLeft` true)
      (`KismetSystemLibrary.PrintString` "isMovedLeftTrue")
      (set `self.isMovedRight` false)
      (`KismetSystemLibrary.PrintString` "IsMovedRight false")
      (if (== (`self.K2_GetActorLocation`) (0.0 0.0 0.0))
        (`KismetSystemLibrary.PrintString` "jau viduryje")
        (set `self.isAtMiddle` true)
        (set `self.IsMovedLeft` false)
        (else
          (set `self.isAtMiddle` false)
          (`KismetSystemLibrary.PrintString` "jau nebe viduryje "))))))

(event `MoveRight`
  ;[1 1 1] Moving to right
  (bind _output_get (set `self.StartLocation` (`self.K2_GetActorLocation`)))
  (bind _output_get_2 (set `self.TargetLocation` (+ _output_get (* (* (`self.GetActorForwardVector`) (-1.0 -1.0 -1.0)) (10.0 10.0 10.0)))))
  (bind (_direction _newtrack_0) (`Timeline|Timeline` :!via `PlayFromStart`)
    (:`Update`
      (`self.K2_SetActorLocation` (`KismetMathLibrary.VLerp` _output_get _output_get_2 _newtrack_0)))
    (:`Finished`
      (set `self.IsMovedLeft` false)
      (`KismetSystemLibrary.PrintString` "isMovedLeftTrue")
      (set `self.isMovedRight` true)
      (`KismetSystemLibrary.PrintString` "IsMovedRight false")
      (if (== (`self.K2_GetActorLocation`) (0.0 0.0 0.0))
        (`KismetSystemLibrary.PrintString` "jau viduryje")
        (set `self.isAtMiddle` true)
        (set `self.isMovedRight` false)
        (else
          (`KismetSystemLibrary.PrintString` "jau nebe viduryje ")
          (set `self.isAtMiddle` false))))))

(event `Jump`
  (bind _output_get (set `self.StartLocation` (`self.K2_GetActorLocation`)))
  (bind _output_get_2 (set `self.TargetLocation` (+ _output_get (* (`self.GetActorUpVector`) (16.0 16.0 16.0)))))
  (set `self.IsJumping` true)
  (bind (_direction _newtrack_0) (`Timeline|JumpTimeline` :!via `PlayFromStart`)
    (:`Update`
      (`self.K2_SetActorLocation` (`KismetMathLibrary.VLerp` _output_get _output_get_2 _newtrack_0)))
    (:`Finished`
      (set `self.IsJumping` false))))

(fn `NewFunction`)

(fn `PhotoAnimation`
  (`SkeletalMeshComponent.PlayAnimation` (`self.SK_Mannequin`) "/Game/MCO_Mocap_Basics/Animation/Walks/In_Place/Walk_02_Cheerful_Loop_IP.Walk_02_Cheerful_Loop_IP" false))

(fn `UserConstructionScript`)